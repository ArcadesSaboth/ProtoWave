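; Van AI vehicle Blueprint, a child class that supplies van-specific body parts to its parent's logic.
; InitRefs fills BodyRefs with the fenders, four wheels and main body (Italian component names), and adds only the main body to the RandomColourizer's mesh list.
; BeginPlay and the construction script just call their parent versions.
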(event `self.ReceiveBeginPlay`
  (`parent.ReceiveBeginPlay`))

(event `self.InitRefs`
  (bind _corpo (`self.corpo`))
  (set `self.bodyRefs` (`|MakeArray` (`self.parafango_poste`) (`self.parafango_ante`) (`self.ruota_ante_dx`) (`self.ruota_ante_sx`) (`self.ruota_poste_dx`) (`self.ruota_poste_sx`) _corpo :!type "PrimitiveComponent Object Reference"))
  (`KismetArrayLibrary.Array_Add` (`/Game/Blueprint/RandomColourizer.meshes` (`self.RandomColourizer`)) _corpo))

(fn `UserConstructionScript`
  (`parent.UserConstructionScript`))