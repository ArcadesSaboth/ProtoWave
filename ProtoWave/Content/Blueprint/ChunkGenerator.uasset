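; Chunk generator actor that builds an endless road along X from sectors, each a run of chunks capped by a crossroad.
; BeginPlay spawns a start road and two sectors from GetRandomSector, advancing a global offset per piece.
; When the player pawn passes NextStart on Tick, it destroys the oldest sector, shifts the second down and appends another.
; It also tracks a semaphore point at the current crossroad, logging when passed.
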(event `ResetGenerator`
  (bind _startroadref (`self.StartRoadRef`))
  (if (!= _startroadref null)
    (`self.K2_DestroyActor` _startroadref))
  (`self.DestroySector` 0)
  (`self.DestroySector` 1)
  (bind _chunkref (`self.SpawnChunkAtNewOffset` (`self.StartRoad`) :!label _label))
  (set `self.StartRoadRef` _chunkref)
  (`KismetArrayLibrary.Array_Add` (`self.SpawnedSector`) (`self.GetRandomSector`))
  (`KismetArrayLibrary.Array_Add` (`self.SpawnedSector`) (`self.GetRandomSector`))
  (for (_array_element _array_index) (`self.SpawnedSector`)
    (bind (_chunks _crossroad) (break `/Game/Blueprint/Sector` _array_element))
    (for (_array_element_2 _array_index_2) _chunks
      (bind _chunkref_2 (`self.SpawnChunkAtNewOffset` _array_element_2))
      (`self.SetFirstNextStart` _array_index_2 _array_index)
      (`KismetArrayLibrary.Array_Add` (`self.TempChunksRef`) _chunkref_2))
    (bind _chunkref_3 (`self.SpawnChunkAtNewOffset` _crossroad))
    (bind _output_get (set `self.TempCrossroadRef` _chunkref_3))
    (`self.SetInitialSemaphore` _output_get _array_index)
    (`KismetArrayLibrary.Array_Set` (`self.SpawnedSector`) _array_index (make `/Game/Blueprint/Sector` _chunks _crossroad (`self.TempChunksRef`) (`self.TempCrossroadRef`)))))

(event `self.ReceiveBeginPlay`
  (goto _label))

(event `self.ReceiveTick`
  (params (DeltaSeconds :type "Float (single-precision)"))
  (if (>= (`KismetMathLibrary.FTrunc` (.x (`self.K2_GetActorLocation` (`GameplayStatics.GetPlayerPawn` 0)))) (`self.NextStart`))
    (`self.GeneraNuovoSector`))
  (if (and (>= (`KismetMathLibrary.FTrunc` (.x (`self.K2_GetActorLocation` (`GameplayStatics.GetPlayerPawn` 0)))) (`self.NextSemaphore`)) (not (`self.NextSemaphorePassed`)))
    (set `self.NextSemaphorePassed` true)
    (`/Game/Blueprint/ProtoWaveUtils.LogInfo` "Semaphore Passed")))

(fn `CalcoloOffset`
  (returns (OffsetPosition :type "Vector Structure"))
  (bind _returnvalue (+ (`self.ChunkXOffset`) (`self.GlobalOffsetPosition`)))
  (set `self.GlobalOffsetPosition` _returnvalue)
  (return (`KismetMathLibrary.MakeVector` (`KismetMathLibrary.Conv_IntToDouble` _returnvalue))))

(fn `DestroySector`
  (params (SectorIndex :type Integer :default 0))
  (bind (_item_chunks _item_crossroad _item_chunksref _item_crossroadref) (break `/Game/Blueprint/Sector` (`KismetArrayLibrary.Array_Get` (`self.SpawnedSector`) SectorIndex)))
  (for _array_element _item_chunksref
    (`/Engine/EditorBlueprintResources/StandardMacros.IsValid` _array_element
      (:`Is Valid`
        (`self.K2_DestroyActor` _array_element))))
  (`/Engine/EditorBlueprintResources/StandardMacros.IsValid` _item_crossroadref
    (:`Is Valid`
      (`self.K2_DestroyActor` _item_crossroadref))))

(fn `GeneraNuovoSector`
  (bind _spawnedsector (`self.SpawnedSector`))
  (bind _startroadref (`self.StartRoadRef`))
  (bind (_chunks _crossroad) (break `/Game/Blueprint/Sector` (`self.GetRandomSector`)))
  (bind _item (`KismetArrayLibrary.Array_Get` _spawnedsector 1))
  (`/Engine/EditorBlueprintResources/StandardMacros.IsValid` _startroadref
    (:`Is Valid`
      (`self.K2_DestroyActor` _startroadref))
    (:`Is Not Valid`
      _))
  (`self.DestroySector` 0)
  (`KismetArrayLibrary.Array_Set` _spawnedsector 0 _item)
  (`self.SetSemaphore` (`.CrossroadRef_34_7E266B60483BA6B8E5A6B9A8626256EB` (break `/Game/Blueprint/Sector` _item)))
  (bind (_chunksref _crossroadref) (`self.InstantiateSector` _chunks _crossroad))
  (`KismetArrayLibrary.Array_Set` (`self.SpawnedSector`) 1 (make `/Game/Blueprint/Sector` _chunks _crossroad _chunksref _crossroadref)))

(fn `InstantiateSector`
  (params (Chunks :type "Array of /Game/Blueprint/Chunk Class Reference") (Crossroad :type "Actor Class Reference"))
  (returns (ChunksRef :type "Array of Actor Object Reference") (CrossRoadRef :type "Actor Object Reference"))
  (for (_array_element _array_index) Chunks
    (bind _chunkref (`self.SpawnChunkAtNewOffset` _array_element))
    (`KismetArrayLibrary.Array_Add` (`self.TempChunksRef`) _chunkref)
    (`self.SetNextStart` _array_index))
  (bind _chunkref_2 (`self.SpawnChunkAtNewOffset` Crossroad))
  (set `self.TempCrossroadRef` _chunkref_2)
  (return (`self.TempChunksRef`) (`self.TempCrossroadRef`)))

(fn `SetFirstNextStart`
  (params (ChunkIndex :type Integer) (SectorIndex :type Integer))
  (if (and (== ChunkIndex (`self.ChunkRegenIndex`)) (== SectorIndex 1))
    (set `self.NextStart` (`self.GlobalOffsetPosition`))))

(fn `SetInitialSemaphore`
  (params (SelfCrossroad :type "Actor Object Reference") (SectorIndex :type Integer))
  (if (== SectorIndex 0)
    (`self.SetSemaphore` SelfCrossroad)))

(fn `SetNextStart`
  (params (ChunkIndex :type Integer))
  (if (== ChunkIndex (`self.ChunkRegenIndex`))
    (set `self.NextStart` (`self.GlobalOffsetPosition`))))

(fn `SetSemaphore`
  (params (InstantiedSemaphore :type "Actor Object Reference"))
  (locals (NewLocalVar_0 :type "Plane Structure"))
  (bind _returnvalue (+ (`KismetMathLibrary.FTrunc` (.x (`self.K2_GetActorLocation` InstantiedSemaphore))) (`self.SemaphoreOffset`)))
  (bind _returnvalue_2 (`KismetMathLibrary.MakeVector` (`KismetMathLibrary.Conv_IntToDouble` _returnvalue) (`self.YSemaphoreOffset`)))
  (set `self.NextSemaphore` _returnvalue)
  (set `self.NextSemaphorePassed` false)
  (`KismetSystemLibrary.DrawDebugSphere` _returnvalue_2 20.0 6 (struct :`G` 0.056797 :`B` 1.0 :`A` 1.0) 1000.0)
  (`/Game/Blueprint/ProtoWaveUtils.LogInfo` (`KismetStringLibrary.Conv_VectorToString` _returnvalue_2)))

(fn `SpawnChunkAtNewOffset`
  (params (Class :type "Actor Class Reference"))
  (returns (ChunkRef :type "Actor Object Reference"))
  (bind _offsetposition (`self.CalcoloOffset`))
  (bind _returnvalue (`|SpawnActorFromClass` Class (`KismetMathLibrary.MakeTransform` _offsetposition (struct :`Yaw` -90.0) (1.0 1.0 1.0)) "Undefined" "OverrideRootScale"))
  (return _returnvalue))

(fn `UserConstructionScript`)