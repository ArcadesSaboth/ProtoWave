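; Game mode that runs the game loop as an enum state machine: Entering, Main Menu, Begin, Play, Dead, Result.
; UI confirms and player spawn/death events advance states, which spawn or clear the player and widgets, start the vehicle spawner and toggle camera follow.
; An interphase pawn is possessed during menu and result screens.
; Tick tracks X distance from PlayerStart, which scores multiplied by caught semaphores plus one.
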(event `self.ReceiveBeginPlay`
  (bind _returnvalue (`|SpawnActorFromClass` "/Game/blueprint/InterphasesPawn.InterphasesPawn_C" (`KismetMathLibrary.MakeTransform` (0.0 0.0 0.0)) "AlwaysSpawn" "OverrideRootScale"))
  (set `self.interphasePawn` _returnvalue)
  (`|ExecutionSequence`
    (:`then_0`
      (bind _outactors (`GameplayStatics.GetAllActorsOfClass` "/Script/Engine.PlayerStart"))
      (if (> (`KismetArrayLibrary.Array_Length` _outactors) 0)
        (set `self.homePoint` (`self.K2_GetActorLocation` (`KismetArrayLibrary.Array_Get` _outactors)))
        (else
          (`/Game/Blueprint/ProtoWaveUtils.LogWarning` "No PlayerStart has been found. Homepoint will be set at origin." self))))
    (:`then_1`
      (bind _returnvalue_2 (`|SpawnActorFromClass` "/Game/blueprint/PlayerCameraFollower.PlayerCameraFollower_C" (`KismetMathLibrary.MakeTransform` (`self.homePoint`)) "AlwaysSpawn" "OverrideRootScale"))
      (set `self.cameraFollowerRef` _returnvalue_2))))

(event `self.ReceiveTick`
  (params (DeltaSeconds :type "Float (single-precision)"))
  ;[1 1 1] Update Logic
  (`self.UpdateFSM`))

(event `/Game/blueprint/GameModeLogic.UIConfirm`
  ;[1 1 1] Confirmation from InterphasePawn
  (switch `/Game/blueprint/gm_states_t` (`self.currentStatus`)
    (:`NewEnumerator0`
      _)
    (:`NewEnumerator4`
      _))
  (`self.NextState`))

(event `/Game/blueprint/GameModeLogic.OnPlayerEndSpawnAnimation`
  (bind _currentstatus (`self.currentStatus`))
  ;[1 1 1] Player Events
  (if (`|EnumEquality` _currentstatus "NewEnumerator1")
    (`self.NextState`)
    (else
      (`/Game/Blueprint/ProtoWaveUtils.LogError` (`KismetStringLibrary.Concat_StrStr` "Player End Spawn during wrong state of:" (`|GetEnumeratorNameAsString` _currentstatus)) self))))

(event `/Game/blueprint/GameModeLogic.OnPlayerBeginDeath`
  (bind _currentstatus (`self.currentStatus`))
  ;[1 1 1] Player Events
  (if (`|EnumEquality` _currentstatus "NewEnumerator2")
    (`self.NextState`)
    (else
      (`/Game/Blueprint/ProtoWaveUtils.LogError` (`KismetStringLibrary.Concat_StrStr` "Player Death during wrong state of:" (`|GetEnumeratorNameAsString` _currentstatus)) self))))

(event `/Game/blueprint/GameModeLogic.OnPlayerEndDeath`
  (bind _currentstatus (`self.currentStatus`))
  ;[1 1 1] Player Events
  (if (`|EnumEquality` _currentstatus "NewEnumerator3")
    (`self.NextState`)
    (else
      (`/Game/Blueprint/ProtoWaveUtils.LogError` (`KismetStringLibrary.Concat_StrStr` "Player End Death during wrong state of:" (`|GetEnumeratorNameAsString` _currentstatus)) self))))

(fn `ActivateSpawner`
  (bind _outactors (`GameplayStatics.GetAllActorsOfClass` "/Game/blueprint/VehicleSpawnerTuaMadre.VehicleSpawnerTuaMadre_C"))
  (`/Game/blueprint/VehicleSpawnerTuaMadre.StartSpawning` (`KismetArrayLibrary.Array_Get` _outactors)))

(fn `ClearPlayer`
  (bind _playerpawn (`self.playerPawn`))
  (`/Engine/EditorBlueprintResources/StandardMacros.IsValid` _playerpawn
    (:`Is Valid`
      (`self.K2_DestroyActor` _playerpawn))))

(fn `ClearWidget`
  (bind _currentui (`self.currentUI`))
  (`/Engine/EditorBlueprintResources/StandardMacros.IsValid` _currentui
    (:`Is Valid`
      (`Widget.RemoveFromParent` _currentui))))

(fn `GetActualScore`
  (returns (score :type Integer))
  (return (`KismetMathLibrary.FTrunc` (* (+ (`self.catchedSemaphores`) 1) (`self.distance`)))))

(fn `NextState`
  (switch `/Game/blueprint/gm_states_t` (`self.currentStatus`)
    (:`NewEnumerator5`
      ;[1 1 1] Entering -> MainMenu
      (set `self.currentStatus` "NewEnumerator0")
      (`Controller.Possess` (`GameplayStatics.GetPlayerController` 0) (`self.interphasePawn`)))
    (:`NewEnumerator0`
      (set `self.currentStatus` "NewEnumerator1")
      (`self.SpawnPlayer`)
      (`self.ClearWidget`)
      (`self.ActivateSpawner`))
    (:`NewEnumerator1`
      (set `self.currentStatus` "NewEnumerator2")
      (set `self.distance` 0.0)
      (set `self.catchedSemaphores` 0))
    (:`NewEnumerator2`
      (set `self.currentStatus` "NewEnumerator3")
      (`/Game/blueprint/PlayerCameraFollower.EnableFollow` (`self.cameraFollowerRef`) false))
    (:`NewEnumerator3`
      (set `self.currentStatus` "NewEnumerator4")
      (`self.ClearPlayer`)
      (`self.SpawnWidget` "/Game/UI/ProtoResultScreen.ProtoResultScreen_C")
      (`Controller.Possess` (`GameplayStatics.GetPlayerController` 0) (`self.interphasePawn`)))
    (:`NewEnumerator4`
      ;[1 1 1] Result -> MainMenu
      (set `self.currentStatus` "NewEnumerator0")
      (`Controller.Possess` (`GameplayStatics.GetPlayerController` 0) (`self.interphasePawn`)))))

(fn `SpawnPlayer`
  (bind _playerpawn (`self.playerPawn`))
  (bind _camerafollowerref (`self.cameraFollowerRef`))
  (`|ExecutionSequence`
    (:`then_0`
      (`/Engine/EditorBlueprintResources/StandardMacros.IsValid` _playerpawn
        (:`Is Valid`
          (`self.K2_DestroyActor` _playerpawn))))
    (:`then_1`
      (bind _returnvalue (`|SpawnActorFromClass` (`self.playerClass`) (`KismetMathLibrary.MakeTransform` (`self.homePoint`) (`KismetMathLibrary.Conv_VectorToRotator` (`self.worldDirection`)) (1.0 1.0 1.0)) "AlwaysSpawn" "OverrideRootScale"))
      (bind _output_get (set `self.playerPawn` _returnvalue))
      (`Controller.Possess` (`GameplayStatics.GetPlayerController` 0) _output_get)
      (set `/Game/blueprint/PlayerCameraFollower.followed` _output_get _camerafollowerref)
      (`/Game/blueprint/PlayerCameraFollower.EnableFollow` _camerafollowerref true))))

(fn `SpawnWidget`
  (params (widgetclass :type "UserWidget Class Reference"))
  (bind _currentui (`self.currentUI`))
  (`|ExecutionSequence`
    (:`then_0`
      (`/Engine/EditorBlueprintResources/StandardMacros.IsValid` _currentui
        (:`Is Valid`
          (`Widget.RemoveFromParent` _currentui))))
    (:`then_1`
      (bind _returnvalue (`|CreateWidget` widgetclass))
      (bind _output_get (set `self.currentUI` _returnvalue))
      (`UserWidget.AddToViewport` _output_get 0))))

(fn `UpdateBeginAnimation`)

(fn `UpdateDeath`)

(fn `UpdateEntering`
  (`self.SpawnWidget` "/Game/UI/ProtoMainMenuGame.ProtoMainMenuGame_C")
  (`self.NextState`))

(fn `UpdateFSM`
  (switch `/Game/blueprint/gm_states_t` (`self.currentStatus`)
    (:`NewEnumerator5`
      (`self.UpdateEntering`))
    (:`NewEnumerator0`
      (`self.UpdateMainMenu`))
    (:`NewEnumerator1`
      (`self.UpdateBeginAnimation`))
    (:`NewEnumerator2`
      (`self.UpdateGame` 0.0))
    (:`NewEnumerator3`
      (`self.UpdateDeath`))
    (:`NewEnumerator4`
      (`self.UpdateResultScreen`))))

(fn `UpdateGame`
  (params (deltaTime :type "Float (double-precision)"))
  (bind _homepoint_x (`KismetMathLibrary.BreakVector` (`self.homePoint`)))
  (bind _returnvalue_x (`KismetMathLibrary.BreakVector` (`self.K2_GetActorLocation` (`self.playerPawn`))))
  (set `self.distance` (`KismetMathLibrary.Abs` (- _returnvalue_x _homepoint_x))))

(fn `UpdateMainMenu`)

(fn `UpdateResultScreen`)

(fn `UserConstructionScript`)