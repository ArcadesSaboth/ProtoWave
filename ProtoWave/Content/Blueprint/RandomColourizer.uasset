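; RandomColourizer is a Blueprint that gives a set of meshes random colours from a palette.
; Its Colourize function loops over the Meshes array and replaces each material in slot 0 with a dynamic instance of that material.
; It then sets the instance's "Colour" vector parameter to a random entry from the Colours array, picked independently for each mesh.
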(fn `Colourize`
  (bind _colours (`self.colours`))
  (for _array_element (`self.meshes`)
    (bind _returnvalue (`PrimitiveComponent.CreateDynamicMaterialInstance` _array_element 0 (`PrimitiveComponent.GetMaterial` _array_element 0)))
    (`PrimitiveComponent.SetMaterial` _array_element 0 _returnvalue)
    (`MaterialInstanceDynamic.SetVectorParameterValue` _returnvalue "Colour" (`KismetArrayLibrary.Array_Get` _colours (`KismetMathLibrary.RandomIntegerInRange` 0 (- (`KismetArrayLibrary.Array_Length` _colours) 1))))))