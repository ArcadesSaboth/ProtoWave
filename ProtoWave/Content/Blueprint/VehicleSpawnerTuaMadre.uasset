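; Spawns and culls AI traffic cars in a moving window around the player, measured along the GameFlowMarker's forward axis.
; Once StartSpawning enables it, each Tick registers new SpawnMarkers as lanes, each with a vehicle queue and two MarkerAI actors.
; Vehicles outside the window are destroyed.
; The MarkerAI pair tracks the last covered bounds, so cars spawn only in newly exposed ranges, at fixed steps with random chance.
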(event `self.ReceiveBeginPlay`)

(event `StartSpawning`
  (`self.Setup`))

(event `self.ReceiveTick`
  (params (DeltaSeconds :type "Float (single-precision)"))
  (if (`self.Enabled`)
    (`self.CatchNewMarkers`)
    (`self.ClearVehicles`)
    (`self.SpawnVehicles`)))

(fn `AddToMarkerQueue`
  (params (Marker :type "/Game/blueprint/SpawnMarker Object Reference") (NewVehicle :type "/Game/Blueprint/Vehicle_AI Object Reference"))
  (for _array_element (`self.VehicleQueues`)
    (bind (_marker _spawnedvehicles) (break `/Game/Blueprint/VehicleQueue` _array_element))
    (if (== Marker _marker)
      (`KismetArrayLibrary.Array_Add` _spawnedvehicles NewVehicle)
      (return))))

(fn `CatchNewMarkers`
  (bind _outactors (`GameplayStatics.GetAllActorsOfClass` "/Game/blueprint/SpawnMarker.SpawnMarker_C"))
  (for _array_element _outactors
    (bind _isnew (`self.IsNewMarker` _array_element))
    (if _isnew
      (bind _vehiclequeue (`self.NewVehicleQueue` _array_element))
      (`KismetArrayLibrary.Array_Add` (`self.VehicleQueues`) _vehiclequeue))))

(fn `ClearVehicles`
  (bind (_beginspawn _playerpos _endspawn) (`self.GetSpawnArea`))
  (for _array_element (`self.VehicleQueues`)
    (for _array_element_2 (`.SpawnedVehicles_8_B07C852147A3BD42107DA1884C65C261` (break `/Game/Blueprint/VehicleQueue` _array_element))
      (bind _returnvalue (`KismetMathLibrary.Dot_VectorVector` (`self.K2_GetActorLocation` _array_element_2) (`self.GetGameFlow`)))
      (if (or (< _returnvalue _beginspawn) (> _returnvalue _endspawn))
        (`self.K2_DestroyActor` _array_element_2)))))

(fn `IsNewMarker`
  (params (Marker :type "/Game/blueprint/SpawnMarker Object Reference"))
  (returns (IsNew :type Boolean))
  (for _array_element (`self.VehicleQueues`)
    (if (== Marker (`.Marker_14_7E5DB89C4193531209B68D89A7A14099` (break `/Game/Blueprint/VehicleQueue` _array_element)))
      (return false)))
  (return true))

(fn `NewVehicleQueue`
  (params (Marker :type "/Game/blueprint/SpawnMarker Object Reference"))
  (returns (VehicleQueue :type "/Game/Blueprint/VehicleQueue Structure"))
  (bind _returnvalue (`KismetMathLibrary.MakeTransform` (+ (`self.K2_GetActorLocation` Marker) (* (`self.GetGameFlow`) (`.PlayerPos` (`self.GetSpawnArea`)))) (`KismetMathLibrary.Conv_VectorToRotator` (`self.GetMarkerDir` Marker))))
  (bind _returnvalue_2 (`|SpawnActorFromClass` "/Game/Blueprint/MarkerAI.MarkerAI_C" _returnvalue "AlwaysSpawn" "OverrideRootScale"))
  (bind _returnvalue_3 (`|SpawnActorFromClass` "/Game/Blueprint/MarkerAI.MarkerAI_C" _returnvalue "AlwaysSpawn" "OverrideRootScale"))
  (return (make `/Game/Blueprint/VehicleQueue` Marker (`|MakeArray`) _returnvalue_2 _returnvalue_3)))

(fn `Setup`
  (`|ExecutionSequence`
    (:`then_0`
      ;[1 1 1] Player
      (bind _outactors (`GameplayStatics.GetAllActorsOfClass` "/Game/blueprint/ProtoPlayer.ProtoPlayer_C"))
      (set `self.Player` (`KismetArrayLibrary.Array_Get` _outactors)))
    (:`then_1`
      ;[1 1 1] GameFlow
      (bind _outactors_2 (`GameplayStatics.GetAllActorsOfClass` "/Game/blueprint/GameFlowMarker.GameFlowMarker_C"))
      (set `self.GameFlow` (`KismetArrayLibrary.Array_Get` _outactors_2)))
    (:`then_2`
      ;[1 1 1] Activate
      (set `self.Enabled` true))))

(fn `SpawnOnRange`
  (params (Marker :type "/Game/blueprint/SpawnMarker Object Reference") (StartSpawn :type "Float (double-precision)") (EndSpawn :type "Float (double-precision)"))
  (for _index (range (+ (`KismetMathLibrary.Round` (/ (- EndSpawn StartSpawn) (`self.SpawnStep`))) 1))
    (if (> _index 0)
      (if (< (`KismetMathLibrary.RandomFloat`) (`self.SpawnChance`))
        (bind _returnvalue (`|SpawnActorFromClass` "/Game/Blueprint/Car_AI.Car_AI_C" (`self.GetTransformAtLocation` Marker (+ (* _index (`self.SpawnStep`)) StartSpawn)) "Undefined" "OverrideRootScale"))
        (`self.AddToMarkerQueue` Marker _returnvalue)))))

(fn `SpawnVehicles`
  (bind (_beginspawn _playerpos _endspawn) (`self.GetSpawnArea`))
  (bind _gameflow (`self.GetGameFlow`))
  (for _array_element (`self.VehicleQueues`)
    (bind (_marker _spawnedvehicles _beginmarkerai _endmarkerai) (break `/Game/Blueprint/VehicleQueue` _array_element))
    (`self.SpawnOnRange` _marker _beginspawn (`KismetMathLibrary.Dot_VectorVector` (`self.K2_GetActorLocation` _beginmarkerai) _gameflow))
    (`self.SpawnOnRange` _marker (`KismetMathLibrary.Dot_VectorVector` _gameflow (`self.K2_GetActorLocation` _endmarkerai)) _endspawn)
    (`self.SyncMarkersAI` _array_element)))

(fn `SyncMarkersAI`
  (params (VehicleQueue :type "/Game/Blueprint/VehicleQueue Structure"))
  (bind (_marker _spawnedvehicles _beginmarkerai _endmarkerai) (break `/Game/Blueprint/VehicleQueue` VehicleQueue))
  (bind (_beginspawn _playerpos _endspawn) (`self.GetSpawnArea`))
  (`self.K2_SetActorTransform` _beginmarkerai (`self.GetTransformAtLocation` null _beginspawn) false true)
  (`self.K2_SetActorTransform` _endmarkerai (`self.GetTransformAtLocation` null _endspawn) false true))

(fn `UserConstructionScript`)