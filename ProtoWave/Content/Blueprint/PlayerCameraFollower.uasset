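; PlayerCameraFollower is a camera actor that becomes the first player's view target at BeginPlay and follows a target actor horizontally along the world X axis.
; Each tick, while the Follow flag is on, it moves its root to the Followed actor's X position and keeps its own Y and Z.
; The EnableFollow event lets other code switch the tracking on or off.
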(event `self.ReceiveBeginPlay`
  (`PlayerController.SetViewTargetWithBlend` (`GameplayStatics.GetPlayerController` 0) self 0.0 "VTBlend_Linear" 0.0 false))

(event `self.ReceiveTick`
  (params (DeltaSeconds :type "Float (single-precision)"))
  (bind (_returnvalue_x _returnvalue_y _returnvalue_z) (`KismetMathLibrary.BreakVector` (`self.K2_GetActorLocation`)))
  (bind _returnvalue_x_2 (`KismetMathLibrary.BreakVector` (`self.K2_GetActorLocation` (`self.followed`))))
  (if (`self.follow`)
    (`SceneComponent.K2_SetWorldLocation` (`self.DefaultSceneRoot`) (`KismetMathLibrary.MakeVector` _returnvalue_x_2 _returnvalue_y _returnvalue_z) false false)))

(event `EnableFollow`
  (params (value :type Boolean))
  (set `self.follow` value))

(fn `UserConstructionScript`)