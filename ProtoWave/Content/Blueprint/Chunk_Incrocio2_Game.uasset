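; Level chunk Blueprint for a crossroads (incrocio) variant, with minion spawns and a semaphore (traffic light) collider.
; On BeginPlay it registers five guaranteed minion spawns, each defined by a begin and end static mesh pair, without calling the parent BeginPlay.
; When the ProtoPlayer hits the semaphore collider, the game mode adds a "semaphore catched" message.
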(event `self.SemaphoreCollider.OnComponentHit`
  (params (HitComponent :type "PrimitiveComponent Object Reference") (OtherActor :type "Actor Object Reference") (OtherComp :type "PrimitiveComponent Object Reference") (NormalImpulse :type "Vector Structure") (Hit :type "HitResult Structure (by ref)"))
  (cast `/Game/blueprint/ProtoPlayer` OtherActor)
  (message `/Game/blueprint/GameModeLogic.AddSemaphoreCatched` (`GameplayStatics.GetGameMode`)))

(event `self.ReceiveBeginPlay`
  (`self.AddMinionSpawnFromStaticMeshes` (`self.Begin Spawn 1`) (`self.End Spawn 1`) 100.0)
  (`self.AddMinionSpawnFromStaticMeshes` (`self.Begin Spawn 2`) (`self.End Spawn 2`) 100.0)
  (`self.AddMinionSpawnFromStaticMeshes` (`self.Begin Spawn 3`) (`self.End Spawn 3`) 100.0)
  (`self.AddMinionSpawnFromStaticMeshes` (`self.Begin Spawn 4`) (`self.End Spawn 4`) 100.0)
  (`self.AddMinionSpawnFromStaticMeshes` (`self.Begin Spawn 5`) (`self.End Spawn 5`) 100.0))

(fn `UserConstructionScript`
  (`parent.UserConstructionScript`))