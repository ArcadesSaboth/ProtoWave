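; Graviter is a component that computes a ground-following, gravity-affected transform for its owner, exposed through a getter rather than applied directly.
; Each Update consumes accumulated movement deltas; single-point mode raycasts from slope height, snapping up on climbs or falling at constant gravity speed.
; Two-point mode derives centre and look-at rotation from two temporary positions, but the logic that grounds those positions is disconnected.
; Debug spheres show the result.
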(event `self.ReceiveBeginPlay`
  (bind _returnvalue (`self.GetOwner`))
  (`KismetArrayLibrary.Array_Add` (`self.ignoreParent`) _returnvalue)
  (`self.TransformFromPoint` (`Actor.K2_GetActorLocation` _returnvalue)))

(event `Update`
  (params (deltaTIme :type "Float (double-precision)"))
  (bind _actualtransform_location (`KismetMathLibrary.BreakTransform` (`self.actualTransform`)))
  (`|ExecutionSequence`
    (:`then_0`
      (if (`self.initialized`)
        (`self.SingleRaycastUpdate` deltaTIme)
        (else
          (`self.DoubleRaycastUpdate` deltaTIme)))
      (`KismetSystemLibrary.DrawDebugSphere` _actualtransform_location 100.0 12 (struct :`R` 0.244418 :`G` 0.165496 :`B` 1.0 :`A` 1.0)))
    (:`then_1`
      (set `self.deltaMovementThisFrame` (0.0 0.0 0.0)))))

(fn `AddDeltaMovement`
  (params (worldDeltaMovement :type "Vector Structure"))
  (set `self.deltaMovementThisFrame` (+ worldDeltaMovement (`self.deltaMovementThisFrame`))))

(fn `DoubleRaycastUpdate`
  (params (deltaTime :type "Float (double-precision)"))
  (locals (firstProjectedCast :type "Vector Structure") (secondProjectedCast :type "Vector Structure") (tempPositionFirst :type "Vector Structure") (tempPositionSecond :type "Vector Structure") (firstPlusMovement :type "Vector Structure") (secondPlusMovement :type "Vector Structure"))
  (bind _temppositionfirst (`local.tempPositionFirst`))
  (bind _temppositionsecond (`local.tempPositionSecond`))
  (`|ExecutionSequence`
    (:`then_0`
      ;[1 1 1] Add movement to both points and cast them to world space
      (bind _result (`self.RelativeToWorldAndMovement` (`self.raycastPoint`) (`self.deltaMovementThisFrame`)))
      (set `local.firstPlusMovement` _result)
      (bind _result_2 (`self.RelativeToWorldAndMovement` (`self.secondRelativePoint`) (`self.deltaMovementThisFrame`)))
      (set `local.secondPlusMovement` _result_2))
    (:`then_1`)
    (:`then_2`)
    (:`then_3`
      (bind _center (`self.WorldCenter` _temppositionfirst _temppositionsecond))
      (set `self.actualTransform` (`KismetMathLibrary.MakeTransform` _center (`KismetMathLibrary.FindLookAtRotation` _temppositionfirst _temppositionsecond))))))

(fn `GetCalculatedWorldTransform`
  (returns (worldTransform :type "Transform Structure"))
  (return (`self.actualTransform`)))

(fn `Init`
  (params (first :type "PrimitiveComponent Object Reference"))
  (set `self.raycastPoint` (`SceneComponent.RelativeLocation` first))
  (set `self.initialized` true))

(fn `RaycastFrom`
  (params (worldLocation :type "Vector Structure"))
  (returns (raycastedWorldLocation :type "Vector Structure") (hit :type Boolean))
  (bind _outhit (`KismetSystemLibrary.LineTraceSingleForObjects` (+ worldLocation (`self.slopeMaxHeight`)) (+ worldLocation (* (`self.raycastDirection`) 1000.0)) (`self.collisionChannels`) false (`self.ignoreParent`) "None" false))
  (return (`.Location` (`GameplayStatics.BreakHitResult` _outhit)) (`GameplayStatics.BreakHitResult` _outhit)))

(fn `RaycastOrCompensateWorldPoint`
  (params (worldLocation :type "Vector Structure") (projectedCast :type "Vector Structure (by ref)"))
  (bind (_raycastedworldlocation _hit) (`self.RaycastFrom` worldLocation))
  (`|VariableSetRef` projectedCast _raycastedworldlocation)
  (if (not _hit)
    (`|VariableSetRef` projectedCast (- worldLocation (0.0 0.0 1000.0))))
  (return))

(fn `RelativeToWorldAndMovement`
  (params (relativePosition :type "Vector Structure") (deltaWorldMovement :type "Vector Structure"))
  (returns (result :type "Vector Structure"))
  (return (+ deltaWorldMovement (`KismetMathLibrary.TransformLocation` (`Actor.GetTransform` (`self.GetOwner`)) relativePosition))))

(fn `SetRaycastersFromRelativeComponent`
  (params (first :type "PrimitiveComponent Object Reference") (second :type "PrimitiveComponent Object Reference"))
  (set `self.raycastPoint` (`SceneComponent.RelativeLocation` first))
  (set `self.secondRelativePoint` (`SceneComponent.RelativeLocation` second))
  (set `self.initialized` false))

(fn `SingleRaycastUpdate`
  (params (deltaTime :type "Float (double-precision)"))
  (locals (projectedCast :type "Vector Structure"))
  (bind (_actualtransform_location _actualtransform_rotation _actualtransform_scale) (`KismetMathLibrary.BreakTransform` (`self.actualTransform`)))
  (bind (_projectedcast_x _projectedcast_y _projectedcast_z) (`KismetMathLibrary.BreakVector` (`local.projectedCast`)))
  (bind _result (`self.RelativeToWorldAndMovement` (`self.raycastPoint`) (`self.deltaMovementThisFrame`)))
  (`self.RaycastOrCompensateWorldPoint` _result (`local.projectedCast`))
  (if (>= _projectedcast_z (`self.CurrentZ`))
    ;[1 1 1] In case the ray cast is above us we instantly move our point there
    ; (it means we are climbing a slope)
    (set `self.actualTransform` (`KismetMathLibrary.MakeTransform` (`local.projectedCast`) (`self.OwnerRotation`)))
    (else
      ;[1 1 1] Raycasted point is below us, so we apply gravity
      (set `self.actualTransform` (`KismetMathLibrary.MakeTransform` (+ (* (`self.gravity`) deltaTime) _actualtransform_location) (`self.OwnerRotation`) _actualtransform_scale)))))

(fn `TransformFromPoint`
  (params (point :type "Vector Structure"))
  (if (`self.initialized`)
    (set `self.actualTransform` (`KismetMathLibrary.MakeTransform` point (`Actor.K2_GetActorRotation` (`self.GetOwner`))))
    (else
      (set `self.actualTransform` (`KismetMathLibrary.MakeTransform` point (`KismetMathLibrary.FindLookAtRotation` (`self.ToWorld` (`self.raycastPoint`)) (`self.ToWorld` (`self.secondRelativePoint`))))))))

(fn `WorldCenter`
  (params (first :type "Vector Structure") (second :type "Vector Structure"))
  (returns (center :type "Vector Structure"))
  (locals (length :type "Float (double-precision)") (versor :type "Vector Structure"))
  (bind _returnvalue (- second first))
  (set `local.length` (`KismetMathLibrary.VSize` _returnvalue))
  (bind _output_get (set `local.versor` (`KismetMathLibrary.Normal` _returnvalue)))
  (return (+ (* _output_get (/ (`local.length`) 2.0)) first)))