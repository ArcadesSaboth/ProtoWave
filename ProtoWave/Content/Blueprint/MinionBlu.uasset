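; Minion actor Blueprint that switches between walking, idle, a fear-related state and physics ragdoll via the MiniSM integer on Tick.
; UpdateMoving places it along the cached Home-to-Destination line by Timer and switches to idle past TimeToReach, but Tick passes zero delta time.
; Idle and fear states set yellow_blue_bp animation flags once (Feared to false); the last state disables capsule collision and simulates mesh physics.
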(event `self.ReceiveBeginPlay`
  (bind (_returnvalue_x _returnvalue_y _returnvalue_z) (`KismetMathLibrary.BreakVector` (`SceneComponent.K2_GetComponentLocation` (`self.Home`))))
  (bind (_returnvalue_x_2 _returnvalue_y_2) (`KismetMathLibrary.BreakVector` (`SceneComponent.K2_GetComponentLocation` (`self.Destination`))))
  (set `self.cachedHome` (`KismetMathLibrary.MakeVector` _returnvalue_x _returnvalue_y _returnvalue_z))
  (set `self.cachedDestination` (`KismetMathLibrary.MakeVector` _returnvalue_x_2 _returnvalue_y_2 _returnvalue_z)))

(event `self.Capsule.OnComponentBeginOverlap`
  (params (OverlappedComponent :type "PrimitiveComponent Object Reference") (OtherActor :type "Actor Object Reference") (OtherComp :type "PrimitiveComponent Object Reference") (OtherBodyIndex :type Integer) (bFromSweep :type Boolean) (SweepResult :type "HitResult Structure (by ref)")))

(event `self.ReceiveTick`
  (params (DeltaSeconds :type "Float (single-precision)"))
  (bind _minon (`self.Minon`))
  (switch `int` (`self.miniSM`)
    (:`0`
      (`self.UpdateMoving` 0.0))
    (:`1`
      (`/Engine/EditorBlueprintResources/StandardMacros.DoOnce` false
        (:`Completed`
          (bind _asyellow_blue_bp (cast `/Game/assets/Characters/blueprint/yellow_blue_bp` (`SkeletalMeshComponent.GetAnimInstance` (`self.Minon`))))
          (set `/Game/assets/Characters/blueprint/yellow_blue_bp.idled` true _asyellow_blue_bp))))
    (:`2`
      (`/Engine/EditorBlueprintResources/StandardMacros.DoOnce` false
        (:`Completed`
          (bind _asyellow_blue_bp_2 (cast `/Game/assets/Characters/blueprint/yellow_blue_bp` (`SkeletalMeshComponent.GetAnimInstance` (`self.Minon`))))
          (set `/Game/assets/Characters/blueprint/yellow_blue_bp.feared` false _asyellow_blue_bp_2))))
    (:`3`
      (`PrimitiveComponent.SetCollisionEnabled` (`self.Capsule`) "NoCollision")
      (`PrimitiveComponent.SetCollisionEnabled` _minon "PhysicsOnly")
      (`PrimitiveComponent.SetSimulatePhysics` _minon true))))

(fn `UpdateMoving`
  (params (deltaTime :type "Float (double-precision)"))
  (locals (versor :type "Vector Structure"))
  (bind _cachedhome (`self.cachedHome`))
  (bind _output_get (set `self.timer` (+ deltaTime (`self.timer`))))
  (bind _output_get_2 (set `local.versor` (- (`self.cachedDestination`) _cachedhome)))
  (`self.K2_SetActorLocationAndRotation` (+ _cachedhome (* _output_get_2 _output_get)) (`KismetMathLibrary.Conv_VectorToRotator` _output_get_2))
  (if (> (`self.timer`) (`self.timeToReach`))
    (set `self.miniSM` 1)))

(fn `UserConstructionScript`)