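; Car_AI is an AI car Blueprint that supplies its own mesh parts to inherited car logic.
; InitRefs fills BodyRefs with the hood (Cofano), four wheels and body for the explosion effect.
; It also adds the hood and body to the RandomColourizer's mesh list for random colouring.
; BeginPlay and the construction script only call the parent; Tick is disabled.
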(event `self.ReceiveBeginPlay`
  (`parent.ReceiveBeginPlay`))

(event `self.InitRefs`
  (bind _cofano (`self.cofano`))
  (bind _body (`self.body`))
  (bind _meshes (`/Game/Blueprint/RandomColourizer.meshes` (`self.RandomColourizer`)))
  ;[1 1 1] Explosion Effect Initialization
  (set `self.bodyRefs` (`|MakeArray` _cofano (`self.ruota_ante_dx`) (`self.ruota_ante_sx`) (`self.ruota_poste_dx`) (`self.ruota_poste_sx`) _body :!type "PrimitiveComponent Object Reference"))
  ;[1 1 1] Random Colourizer Initialization
  (`KismetArrayLibrary.Array_Add` _meshes _cofano)
  (`KismetArrayLibrary.Array_Add` _meshes _body))

(fn `UserConstructionScript`
  (`parent.UserConstructionScript`))