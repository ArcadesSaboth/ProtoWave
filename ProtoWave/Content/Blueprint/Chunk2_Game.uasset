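; Chunk2_Game is a game chunk Blueprint that registers possible minion spawns within its layout.
; On BeginPlay it calls AddMinionSpawnFromStaticMeshes for five begin and end static mesh marker pairs, each with the same even spawn chance.
; The construction script only runs the parent's version, and the spawn helper's logic is not defined in this graph.
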(event `self.ReceiveBeginPlay`
  (`self.AddMinionSpawnFromStaticMeshes` (`self.BeginSpawn1`) (`self.EndSpawn1`) 50.0)
  (`self.AddMinionSpawnFromStaticMeshes` (`self.BeginSpawn2`) (`self.EndSpawn2`) 50.0)
  (`self.AddMinionSpawnFromStaticMeshes` (`self.BeginSpawn3`) (`self.EndSpawn3`) 50.0)
  (`self.AddMinionSpawnFromStaticMeshes` (`self.BeginSpawn5`) (`self.EndSpawn5`) 50.0)
  (`self.AddMinionSpawnFromStaticMeshes` (`self.BeginSpawn4`) (`self.EndSpawn4`) 50.0))

(fn `UserConstructionScript`
  (`parent.UserConstructionScript`))