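; Base minion that walks from a home point to a destination, then idles, gets scared by the player, or is knocked away on impact.
; A Tick-driven integer state machine handles timed linear movement, then sets idle or fear flags on the anim instance.
; The notifier overlap triggers fear only while moving.
; Capsule overlap with an actor reporting positive speed fakes a hit by switching the mesh to physics and applying an impulse.
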(event `self.ReceiveBeginPlay`
  (bind (_home_x _home_y _home_z) (`KismetMathLibrary.BreakVector` (`self.Home`)))
  (bind (_destination_x _destination_y) (`KismetMathLibrary.BreakVector` (`self.Destination`)))
  ;[1 1 1] Cache variables
  (set `self.cachedHome` (`KismetMathLibrary.MakeVector` _home_x _home_y _home_z))
  (set `self.cachedDestination` (`KismetMathLibrary.MakeVector` _destination_x _destination_y _home_z))
  (set `self.cachedDistance` (`KismetMathLibrary.VSize` (- (`self.cachedDestination`) (`self.cachedHome`)))))

(event `self.Capsule.OnComponentBeginOverlap`
  (params (OverlappedComponent :type "PrimitiveComponent Object Reference") (OtherActor :type "Actor Object Reference") (OtherComp :type "PrimitiveComponent Object Reference") (OtherBodyIndex :type Integer) (bFromSweep :type Boolean) (SweepResult :type "HitResult Structure (by ref)"))
  (bind _minon (`self.Minon`))
  ;[1 1 1] Collision against player (fakes hit)
  (bind _speed (message `/Game/Blueprint/MovableEntity.GetActualSpeed` OtherActor))
  (if (> _speed 0.0)
    (set `self.miniSM` 3)
    (`PrimitiveComponent.SetCollisionEnabled` (`self.Capsule`) "NoCollision")
    (`SkeletalMeshComponent.Stop` _minon)
    (`PrimitiveComponent.SetCollisionEnabled` _minon "PhysicsOnly")
    (`PrimitiveComponent.SetSimulatePhysics` _minon true)
    (`PrimitiveComponent.AddImpulse` _minon (* (`KismetMathLibrary.Normal` (- (`self.K2_GetActorLocation`) (`self.K2_GetActorLocation` OtherActor))) (`self.pushForce`)) "None" false)))

(event `self.PlayerNotifier.OnComponentBeginOverlap`
  (params (OverlappedComponent :type "PrimitiveComponent Object Reference") (OtherActor :type "Actor Object Reference") (OtherComp :type "PrimitiveComponent Object Reference") (OtherBodyIndex :type Integer) (bFromSweep :type Boolean) (SweepResult :type "HitResult Structure (by ref)"))
  ;[1 1 1] Fear on player's sight
  (if (and (`|EnumEquality` (`PrimitiveComponent.GetCollisionObjectType` OtherComp) "ECC_GameTraceChannel1") (== (`self.miniSM`) 0))
    (set `self.miniSM` 2)))

(event `self.ReceiveTick`
  (params (DeltaSeconds :type "Float (single-precision)"))
  ;[1 1 1] State Machine
  (switch `int` (`self.miniSM`)
    (:`0`
      (`self.UpdateMoving` DeltaSeconds))
    (:`1`
      (`/Engine/EditorBlueprintResources/StandardMacros.DoOnce` false
        (:`Completed`
          (bind _asyellow_blue_bp (cast `/Game/assets/Characters/blueprint/yellow_blue_bp` (`SkeletalMeshComponent.GetAnimInstance` (`self.Minon`))))
          (set `/Game/assets/Characters/blueprint/yellow_blue_bp.idled` true _asyellow_blue_bp))))
    (:`2`
      (`/Engine/EditorBlueprintResources/StandardMacros.DoOnce` false
        (:`Completed`
          (bind _asyellow_blue_bp_2 (cast `/Game/assets/Characters/blueprint/yellow_blue_bp` (`SkeletalMeshComponent.GetAnimInstance` (`self.Minon`))))
          (set `/Game/assets/Characters/blueprint/yellow_blue_bp.feared` true _asyellow_blue_bp_2))))))

(fn `UpdateMoving`
  (params (deltaTime :type "Float (double-precision)"))
  (locals (versor :type "Vector Structure"))
  (bind _cachedhome (`self.cachedHome`))
  (bind _output_get (set `self.timer` (+ deltaTime (`self.timer`))))
  (bind _output_get_2 (set `local.versor` (`KismetMathLibrary.Normal` (- (`self.cachedDestination`) _cachedhome))))
  (`SceneComponent.K2_SetWorldLocationAndRotation` (`self.minionRoot`) (+ _cachedhome (* _output_get_2 (* (`self.cachedDistance`) (/ _output_get (`self.timeToReach`))))) (`KismetMathLibrary.Conv_VectorToRotator` _output_get_2) false false)
  (if (> (`self.timer`) (`self.timeToReach`))
    (set `self.miniSM` 1)))

(fn `UserConstructionScript`)