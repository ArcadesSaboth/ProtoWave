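; Crossing pedestrian actor whose skeletal mesh moves back and forth endlessly between two points, A and B.
; On BeginPlay it adds the actor's location to both points, then loops latent MoveComponentTo calls, each lasting NavigationTime.
; At each end SetActorRelativeRotation snaps the actor's facing between 180 and 0 degrees.
; The return move also passes a 180-degree target rotation to the mesh.
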(event `self.ReceiveBeginPlay`
  (bind _returnvalue (`self.K2_GetActorLocation`))
  (bind _skeletalmeshcomponent (`self.SkeletalMeshComponent`))
  (set `self.A` (+ (`self.A`) _returnvalue))
  (set `self.B` (+ (`self.B`) _returnvalue))
  (`KismetSystemLibrary.MoveComponentTo` _skeletalmeshcomponent (`self.B`) (struct) false false (`self.NavigationTime`) :!label _label)
  (`self.K2_SetActorRelativeRotation` (struct :`Yaw` -180.0) false true)
  (`KismetSystemLibrary.MoveComponentTo` _skeletalmeshcomponent (`self.A`) (struct :`Yaw` -180.0) false false (`self.NavigationTime`))
  (`self.K2_SetActorRelativeRotation` (struct) false true)
  (goto _label))

(fn `UserConstructionScript`)