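; TwoPointsGraviter keeps two raycaster components on the surface under them, applying movement and gravity.
; InitReferences stores both components and detaches them from their parents as an admitted workaround.
; Each Update adds the frame's movement delta, projects both points with RaycastOrCompensateWorldPoint, then clears the delta.
; Points snap to projections at or above them; otherwise they move only by Gravity, applied as velocity rather than acceleration.
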(event `self.Update`
  (params (deltaTIme :type "Float (single-precision)"))
  (if (`self.initialized`)
    (`self.UpdateImpl` deltaTIme)
    (set `self.deltaMovementThisFrame` (0.0 0.0 0.0))))

(fn `InitReferences`
  (params (first :type "PrimitiveComponent Object Reference") (second :type "PrimitiveComponent Object Reference"))
  (bind _output_get (set `self.firstRaycasterRef` first))
  (set `self.secondRaycasterRef` second)
  (set `self.initialized` true)
  ;[1 1 1] Detaching them from the parent will prevent a lot of errors but it's a shitty
  ; behaviour. I know it's not good programming but I have enough of this.
  ; Sorry!
  (`SceneComponent.K2_DetachFromComponent` _output_get "KeepWorld" "KeepWorld" "KeepWorld" true)
  (`SceneComponent.K2_DetachFromComponent` second "KeepWorld" "KeepWorld" "KeepWorld" true))

(fn `ProjectedLocationToComponent`
  (params (deltaTIme :type "Float (double-precision)") (component :type "PrimitiveComponent Object Reference (by ref)") (projectedLocation :type "Vector Structure"))
  (bind (_returnvalue_x _returnvalue_y _returnvalue_z) (`KismetMathLibrary.BreakVector` (`SceneComponent.K2_GetComponentLocation` component)))
  (if (>= (.z projectedLocation) _returnvalue_z)
    (`SceneComponent.K2_SetWorldLocation` component projectedLocation false false)
    (else
      ;[1 1 1] Raycasted point is below us, so we apply gravity
      (`SceneComponent.K2_SetWorldLocation` component (+ (* (`self.gravity`) deltaTIme) (`SceneComponent.K2_GetComponentLocation` component)) false false))))

(fn `UpdateImpl`
  (params (deltaTIme :type "Float (double-precision)"))
  (locals (firstLocationAndMovement :type "Vector Structure") (secondLocationAndMovement :type "Vector Structure") (firstProjectedLocation :type "Vector Structure") (secondProjectedLocation :type "Vector Structure"))
  (`|ExecutionSequence`
    (:`then_0`
      ;[1 1 1] Add movement to actual locations
      (set `local.firstLocationAndMovement` (+ (`SceneComponent.K2_GetComponentLocation` (`self.firstRaycasterRef`)) (`self.deltaMovementThisFrame`)))
      (set `local.secondLocationAndMovement` (+ (`SceneComponent.K2_GetComponentLocation` (`self.secondRaycasterRef`)) (`self.deltaMovementThisFrame`))))
    (:`then_1`
      ;[1 1 1] Project location (adjusted by movement)
      (`self.RaycastOrCompensateWorldPoint` (`local.firstLocationAndMovement`) (`local.firstProjectedLocation`))
      (`self.RaycastOrCompensateWorldPoint` (`local.secondLocationAndMovement`) (`local.secondProjectedLocation`)))
    (:`then_2`
      ;[1 1 1] Apply movement and gravity to components
      (`self.ProjectedLocationToComponent` deltaTIme (`self.firstRaycasterRef`) (`local.firstProjectedLocation`))
      (`self.ProjectedLocationToComponent` deltaTIme (`self.secondRaycasterRef`) (`local.secondProjectedLocation`)))))