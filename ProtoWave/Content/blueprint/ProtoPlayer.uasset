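; Player car pawn that drives forward with adjustable speed and strafes within a lateral limit around its spawn point.
; Input presses and releases accumulate a movement vector; Tick turns it into speed, with strafing scaled by forward speed, and feeds the vehicle sound.
; Hard-enemy overlaps trigger a one-time death that blasts car parts apart with physics and notifies the GameMode; soft-enemy overlaps cut speed by a percentage.
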(event `self.ReceiveBeginPlay`
  ;[1 1 1] Initialization
  (set `self.HomePoint` (`self.K2_GetActorLocation`))
  (`self.InitReferences`)
  (message `/Game/blueprint/GameModeLogic.OnPlayerEndSpawnAnimation` (`GameplayStatics.GetGameMode`)))

(event `self.ReceiveTick`
  (params (DeltaSeconds :type "Float (single-precision)"))
  ;[1 1 1] Update
  (`|ExecutionSequence`
    (:`then_0`
      (if (`self.CanMove`)
        (`self.UpdatePosition` DeltaSeconds)
        (`self.InitReferences`)
        (set `/Game/blueprint/SND_Vehicle.Speed` (`self.Speed`) (`self.SND_Vehicle`))))
    (:`then_1`
      (set `self.penaltyTimer` (`KismetMathLibrary.FClamp` (- (`self.penaltyTimer`) DeltaSeconds) 0.0 (`self.EnemySoftPenalyCooldown`))))))

(event `self.Collision.OnComponentBeginOverlap`
  (params (OverlappedComponent :type "PrimitiveComponent Object Reference") (OtherActor :type "Actor Object Reference") (OtherComp :type "PrimitiveComponent Object Reference") (OtherBodyIndex :type Integer) (bFromSweep :type Boolean) (SweepResult :type "HitResult Structure (by ref)"))
  (bind _returnvalue (`PrimitiveComponent.GetCollisionObjectType` OtherComp))
  ;[1 1 1] Collision handling (only against Hard and Sof Enemy)
  (`|ExecutionSequence`
    (:`then_0`
      (if (`|EnumEquality` _returnvalue "ECC_GameTraceChannel2")
        (`/Engine/EditorBlueprintResources/StandardMacros.DoOnce` false
          (:`Completed`
            (`self.Death`)))))
    (:`then_1`
      (if (`|EnumEquality` _returnvalue "ECC_GameTraceChannel3")
        (`self.ApplyEnemySoftPenalty`)))))

(event `InputAction|PlayerBackward`
  (params (Key :type "Key Structure" :default "AnyKey"))
  ;[1 1 1] Input Movements
  (:`Pressed`
    (`self.OffsetMovement` (-1.0 0.0)
      (:`out`
        (if (`self.CanMove`)
          (`/Game/blueprint/SND_Vehicle.Accelerate` (`self.SND_Vehicle`))))))
  (:`Released`
    (`self.OffsetMovement` (1.0 0.0))))

(event `InputAction|PlayerForward`
  (params (Key :type "Key Structure" :default "AnyKey"))
  ;[1 1 1] Input Movements
  (:`Pressed`
    (`self.OffsetMovement` (1.0 0.0)
      (:`out`
        (if (`self.CanMove`)
          (`/Game/blueprint/SND_Vehicle.Brake` (`self.SND_Vehicle`))))))
  (:`Released`
    (`self.OffsetMovement` (-1.0 0.0))))

(event `Death`
  ;[1 1 1] Death handling
  (set `self.CanMove` false)
  (message `/Game/blueprint/GameModeLogic.OnPlayerBeginDeath` (`GameplayStatics.GetGameMode`))
  (`/Game/blueprint/SND_Vehicle.OnDeath` (`self.SND_Vehicle`))
  (for _array_element (`self.carRefs`)
    (`PrimitiveComponent.SetCollisionEnabled` _array_element "PhysicsOnly")
    (`PrimitiveComponent.SetSimulatePhysics` _array_element true)
    (`PrimitiveComponent.AddRadialForce` _array_element (`self.K2_GetActorLocation`) (`self.explosionRadius`) (`self.explosionForce`) "RIF_Constant" false))
  (`KismetSystemLibrary.Delay` (`self.DeathAnimationLength`))
  (message `/Game/blueprint/GameModeLogic.OnPlayerEndDeath` (`GameplayStatics.GetGameMode`)))

(event `InputAction|PlayerLeft`
  (params (Key :type "Key Structure" :default "AnyKey"))
  ;[1 1 1] Input Movements
  (:`Pressed`
    (`self.OffsetMovement` (0.0 -1.0)))
  (:`Released`
    (`self.OffsetMovement` (0.0 1.0))))

(event `InputAction|PlayerRight`
  (params (Key :type "Key Structure" :default "AnyKey"))
  ;[1 1 1] Input Movements
  (:`Pressed`
    (`self.OffsetMovement` (0.0 1.0)))
  (:`Released`
    (`self.OffsetMovement` (0.0 -1.0))))

(event `ApplyEnemySoftPenalty`
  (bind _speed (`self.Speed`))
  (if (> (`self.explosionRadius`) 0.0)
    ;[1 1 1] Decrease the actual speed of a percentage given by
    ; EnemySoftDecelerationPercentage
    (set `self.penaltyTimer` 0.0)
    (set `self.temp` _speed)
    (set `self.Speed` (* _speed (- 1.0 (`self.EnemySoftDecelerationPercentage`))))))

(fn `DrawDebug`
  (bind _uidebug (`self.uidebug`))
  (`/Engine/EditorBlueprintResources/StandardMacros.IsValid` _uidebug
    (:`Is Valid`
      (`TextBlock.SetText` (`/Game/UI/DebugThis.DebugText` _uidebug) (`KismetTextLibrary.Conv_StringToText` (`KismetStringLibrary.Concat_StrStr` "Speed: " (`KismetStringLibrary.Conv_DoubleToString` (`self.Speed`)) "Lateral Speed:" (`KismetStringLibrary.Conv_DoubleToString` (`self.LateralSpeed`))))))))

(fn `GetActualSpeed`
  (returns (speed :type "Float (double-precision)"))
  (return (`self.Speed`)))

(fn `HandleMovement`
  (params (deltaTime :type "Float (double-precision)"))
  (bind (_domovement_x _domovement_y) (`KismetMathLibrary.BreakVector2D` (`self.DoMovement`)))
  (bind _speed (`self.Speed`))
  (`|ExecutionSequence`
    (:`then_0`
      (set `self.LateralSpeed` (* (* (`self.MaxLateralSpeed`) _domovement_y) (/ (`self.Speed`) (`self.MaxSpeed`)))))
    (:`then_1`
      (if (> _domovement_x 0.0)
        (set `self.Speed` (`KismetMathLibrary.FClamp` (+ _speed (* (`self.Acceleration`) deltaTime)) 0.0 (`self.MaxSpeed`)))))
    (:`then_2`
      (if (< _domovement_x 0.0)
        (set `self.Speed` (`KismetMathLibrary.FClamp` (+ _speed (* (`self.Acceleration`) deltaTime -1.0)) 0.0 (`self.MaxSpeed`)))))))

(fn `InitReferences`
  (set `self.carRefs` (`|MakeArray` (`self.cofano`) (`self.sportello_sx`) (`self.sportello_dx`) (`self.ruota_ante_sx`) (`self.ruota_ante_dx`) (`self.ruota_post_sx`) (`self.ruota_post_dx`) (`self.body`))))

(fn `UpdatePosition`
  (params (deltaTime :type "Float (double-precision)"))
  (bind (_returnvalue_x _returnvalue_y _returnvalue_z) (`KismetMathLibrary.BreakVector` (`self.K2_GetActorLocation`)))
  (bind (_direction_x _direction_y) (`KismetMathLibrary.BreakVector` (`self.Direction`)))
  (bind (_homepoint_x _homepoint_y) (`KismetMathLibrary.BreakVector` (`self.HomePoint`)))
  (bind _laterallimit (`self.LateralLimit`))
  (`self.HandleMovement` deltaTime)
  (`self.K2_SetActorLocation` (`KismetMathLibrary.MakeVector` (+ _returnvalue_x (* _direction_x (`self.Speed`))) (`KismetMathLibrary.FClamp` (+ _returnvalue_y (* _direction_y (`self.LateralSpeed`))) (- _homepoint_y _laterallimit) (+ _homepoint_y _laterallimit)) _returnvalue_z)))

(fn `UserConstructionScript`)

(fn `WheelMovement`
  (params (deltaTime :type "Float (double-precision)"))
  (if (`self.CanMove`)
    (for _array_element _
      (`SceneComponent.K2_AddWorldRotation` _array_element (`KismetMathLibrary.RotatorFromAxisAndAngle` (0.0 1.0 0.0) (`self.Speed`)) false false))))