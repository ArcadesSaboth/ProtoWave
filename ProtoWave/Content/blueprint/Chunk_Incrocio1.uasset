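; Chunk_Incrocio1 is a level chunk actor, named as an intersection piece, with almost no active logic.
; Its Box hit event casts the other actor to ProtoPlayer and then does nothing, while BeginPlay and the construction script are empty.
; Disconnected nodes would spawn six Slot actors at offsets from the chunk's location, three per side, with the left row (Lato Sinistro) rotated half a turn, but they never run.
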(event `self.ReceiveBeginPlay`)

(event `self.Box.OnComponentHit`
  (params (HitComponent :type "PrimitiveComponent Object Reference") (OtherActor :type "Actor Object Reference") (OtherComp :type "PrimitiveComponent Object Reference") (NormalImpulse :type "Vector Structure") (Hit :type "HitResult Structure (by ref)"))
  (cast `/Game/blueprint/ProtoPlayer` OtherActor))

(fn `UserConstructionScript`)