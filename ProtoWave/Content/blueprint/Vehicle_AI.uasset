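; AI traffic vehicle that drives in a straight line along its spawn facing, with a randomized body colour.
; Each tick a forward trace finds vehicles ahead, easing speed down on a sine curve as the gap closes.
; Overlap with a specific custom collision channel triggers a one-time death: body parts become physics debris blasted by radial force, and the actor is destroyed after a delay.
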(event `self.ReceiveBeginPlay`
  ;[1 1 1] Initialization
  (set `self.Direction` (`KismetMathLibrary.GetAxes` (`self.K2_GetActorRotation`)))
  (`self.InitRefs`)
  (`self.RandomizeColour`))

(event `self.Box.OnComponentBeginOverlap`
  (params (OverlappedComponent :type "PrimitiveComponent Object Reference") (OtherActor :type "Actor Object Reference") (OtherComp :type "PrimitiveComponent Object Reference") (OtherBodyIndex :type Integer) (bFromSweep :type Boolean) (SweepResult :type "HitResult Structure (by ref)"))
  (`KismetArrayLibrary.Array_AddUnique` (`self.CollisionList`) OtherActor)
  (if (`|EnumEquality` (`PrimitiveComponent.GetCollisionObjectType` OtherComp) "ECC_GameTraceChannel1")
    (`/Engine/EditorBlueprintResources/StandardMacros.DoOnce` false
      (:`Completed`
        (`self.Death`)))))

(event `self.ReceiveActorEndOverlap`
  (params (OtherActor :type "Actor Object Reference"))
  (`KismetArrayLibrary.Array_RemoveItem` (`self.CollisionList`) OtherActor))

(event `self.ReceiveTick`
  (params (DeltaSeconds :type "Float (single-precision)"))
  (bind _mincollisiondistance (`self.MinCollisionDistance`))
  ;[1 1 1] Update
  (if (`self.CanMove`)
    (bind (_iscolliding _distance) (`self.RaycastOtherVehicles`))
    (bind _output_get (set `self.CurrentSpeed` (`KismetMathLibrary.Lerp` 0.0 (`self.Speed`) (`KismetMathLibrary.DegSin` (* (`KismetMathLibrary.FClamp` (/ (- _distance _mincollisiondistance) (- (`self.MaxCollisionDistance`) _mincollisiondistance))) 90.0)))))
    (`SceneComponent.K2_AddWorldOffset` (`self.Box`) (* (`self.Direction`) (* _output_get DeltaSeconds)) false false)
    (set `/Game/blueprint/SND_EnemyVehicle.Speed` (`self.Speed`) (`self.SND_EnemyVehicle`))))

(event `Death`
  ;[1 1 1] Death handling
  (for _array_element (`self.bodyRefs`)
    (`PrimitiveComponent.SetCollisionEnabled` _array_element "PhysicsOnly")
    (`PrimitiveComponent.SetSimulatePhysics` _array_element true)
    (`PrimitiveComponent.AddRadialForce` _array_element (`self.K2_GetActorLocation`) (`self.explosionRadius`) (`self.explosionForce`) "RIF_Constant" false))
  (set `self.CanMove` false)
  (`/Game/blueprint/SND_EnemyVehicle.OnDeath` (`self.SND_EnemyVehicle`))
  (`KismetSystemLibrary.Delay` (`self.deathLength`))
  (`self.K2_DestroyActor`))

(fn `GetActualSpeed`
  (returns (speed :type "Float (double-precision)"))
  (return (`self.Speed`)))

(fn `InitRefs`
  (set `self.bodyRefs` (`|MakeArray` (`self.cofano`) (`self.ruota_ant_dx`) (`self.ruota_ant_sx`) (`self.ruota_post_dx`) (`self.ruota_post_sx`) (`self.body`))))

(fn `IsCollidingObstacles`
  (returns (IsColliding :type Boolean))
  (locals (NumObstaclesAhead :type Integer))
  (set `local.NumObstaclesAhead` 0)
  (for _array_element (`self.CollisionList`)
    (if (> (`KismetMathLibrary.Dot_VectorVector` (- (`self.K2_GetActorLocation` _array_element) (`self.K2_GetActorLocation`)) (`self.Direction`)) 0.0)
      (`KismetSystemLibrary.PrintString` "COLLISION!")
      (return true)))
  (return false))

(fn `RandomizeColour`
  (bind _randomcolourizer (`self.RandomColourizer`))
  (bind _meshes (`/Game/Blueprint/RandomColourizer.meshes` _randomcolourizer))
  (`KismetArrayLibrary.Array_Add` _meshes (`self.body`))
  (`KismetArrayLibrary.Array_Add` _meshes (`self.cofano`))
  (`/Game/Blueprint/RandomColourizer.Colourize` _randomcolourizer))

(fn `RaycastOtherVehicles`
  (returns (IsColliding :type Boolean) (Distance :type "Float (double-precision)"))
  (bind _direction (`self.Direction`))
  (bind _returnvalue (+ (* _direction (.x (`BoxComponent.BoxExtent` (`self.Box`)))) (`self.K2_GetActorLocation`)))
  (bind (_outhit _returnvalue_2) (`KismetSystemLibrary.LineTraceSingleForObjects` :`Start` _returnvalue :`End` (+ _returnvalue (* _direction (`self.RaycastLength`))) :`ObjectTypes` (`|MakeArray` (enumliteral `EObjectTypeQuery` "ObjectTypeQuery8")) :`DrawDebugType` "ForOneFrame"))
  (if _returnvalue_2
    (bind (_bblockinghit _binitialoverlap _time _location _impactpoint _normal _impactnormal _physmat _hitactor _hitcomponent _hitbonename _hititem _faceindex _tracestart) (`GameplayStatics.BreakHitResult` _outhit))
    (return true (`KismetMathLibrary.VSize` (- _location _tracestart)))
    (else
      (return false (`self.MaxCollisionDistance`)))))

(fn `UserConstructionScript`)